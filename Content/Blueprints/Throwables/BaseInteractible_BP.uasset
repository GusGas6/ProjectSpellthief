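; Base throwable interactible that the player can pick up, throw and shatter on impact.
; The construction script builds a static or skeletal mesh component from the assigned model and attaches the grab billboard and range.
; Pickup hands the actor and mesh references to the player, and DisableGravity records thrown velocity.
; Hits above a velocity threshold deal blunt damage and burst into launched gibs; skeletal versions also spawn an EnemySoundActor_BP.
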(event OnComponentBeginOverlap(GrabRange)
  (params (OverlappedComponent :type Primitive%20Component%20Object%20Reference) (OtherActor :type Actor%20Object%20Reference) (OtherComp :type Primitive%20Component%20Object%20Reference) (OtherBodyIndex :type Integer) (bFromSweep :type Boolean) (SweepResult :type Hit%20Result%20Structure%20%28by%20ref%29))
  ;[0.15 0.15 0.15 0.5] Toggle Grab Icon
  (if (== OtherActor (Variables|Default|GetPlayerREF))
    (Development|SetHiddeninGame (Variables|Default|GetGrabBilboard) false false)))

(event OnComponentEndOverlap(GrabRange)
  (params (OverlappedComponent :type Primitive%20Component%20Object%20Reference) (OtherActor :type Actor%20Object%20Reference) (OtherComp :type Primitive%20Component%20Object%20Reference) (OtherBodyIndex :type Integer))
  ;[0.15 0.15 0.15 0.5] Toggle Grab Icon
  (if (== OtherActor (Variables|Default|GetPlayerREF))
    (Development|SetHiddeninGame (Variables|Default|GetGrabBilboard) true false)))

(event OnComponentHit(StaticMeshREF)
  (params (HitComponent :type Primitive%20Component%20Object%20Reference) (OtherActor :type Actor%20Object%20Reference) (OtherComp :type Primitive%20Component%20Object%20Reference) (NormalImpulse :type Vector :default "0, 0, 0") (Hit :type Hit%20Result%20Structure%20%28by%20ref%29))
  (bind _hitactor (Collision|BreakHitResult Hit))
  (bind _staticmeshref (Variables|Default|GetStaticMeshREF))
  (bind _returnvalue (Transformation|GetComponentVelocity _staticmeshref))
  (bind _returnvalue_2 (Math|Vector|VectorLength _returnvalue))
  ;[0.15 0.15 0.15 0.5] On Hit
  (if (>= _returnvalue_2 (Variables|Default|GetMinimumVelocityImpact))
    (Development|PrintString (Utilities|String|ToString(Float) _returnvalue_2))
    (Game|Damage|ApplyPointDamage _hitactor 1.0 (Math|Vector|GetUnitDirection(Vector) (.Location (Collision|BreakHitResult Hit)) (Transformation|GetActorLocation _hitactor)) Hit (Game|GetPlayerController 0) self "/Game/Blueprints/DamageTypes/Blunt_DamageType.Blunt_DamageType_C")
    (CallFunction|Gib false)))

(event OnComponentHit(SkeletalMeshREF)
  (params (HitComponent :type Primitive%20Component%20Object%20Reference) (OtherActor :type Actor%20Object%20Reference) (OtherComp :type Primitive%20Component%20Object%20Reference) (NormalImpulse :type Vector :default "0, 0, 0") (Hit :type Hit%20Result%20Structure%20%28by%20ref%29))
  (bind _hitactor (Collision|BreakHitResult Hit))
  (bind _skeletalmeshref (Variables|Default|GetSkeletalMeshREF))
  (bind _returnvalue (Transformation|GetComponentVelocity _skeletalmeshref))
  (bind _returnvalue_2 (Math|Vector|VectorLength _returnvalue))
  ;[0.15 0.15 0.15 0.5] On Hit
  (if (not (== OtherActor self))
    (if (>= _returnvalue_2 (Variables|Default|GetMinimumVelocityImpact))
      (Development|PrintString (Utilities|String|ToString(Float) _returnvalue_2))
      (Game|Damage|ApplyPointDamage _hitactor 1.0 (Math|Vector|GetUnitDirection(Vector) (.ImpactPoint (Collision|BreakHitResult Hit)) (Transformation|GetActorLocation _hitactor)) Hit (Game|GetPlayerController 0) self "/Game/Blueprints/DamageTypes/Blunt_DamageType.Blunt_DamageType_C")
      (CallFunction|Gib true))))

(event Custom|Gib
  (params (Skeletal :type Boolean))
  (bind _returnvalue (Math|Random|RandomFloatinRange 0.08 0.32))
  (bind _returnvalue_2 (Math|Random|RandomFloatinRange 0.08 0.32))
  (bind _staticmeshref (Variables|Default|GetStaticMeshREF))
  (bind _skeletalmeshref (Variables|Default|GetSkeletalMeshREF))
  (bind _staticmeshref_2 (Variables|Default|GetStaticMeshREF))
  (bind _returnvalue_3 (Transformation|GetWorldLocation _staticmeshref))
  (bind _returnvalue_4 (Transformation|GetWorldLocation _skeletalmeshref))
  ;[0.15 0.15 0.15 0.5] Gib
  (if Skeletal
    (for _index (range 0 5)
      (bind _returnvalue_5 (Game|SpawnActorfromClass "/Game/Blueprints/Gibs/BaseGibs_BP.BaseGibs_BP_C" (Math|Transform|MakeTransform (Math|Vector|MakeVector (.x _returnvalue_4) 0.0 (.z _returnvalue_4)) (Math|Random|RandomRotator false) (Math|Vector|MakeVector _returnvalue_2 _returnvalue_2 _returnvalue_2)) "AlwaysSpawn" "MultiplyWithRoot" 0 0))
      (Physics|AddImpulse (Variables|/Game/Blueprints/Gibs/BaseGibs_BP.BaseGibs_BP_C|GetBaseGibMesh _returnvalue_5) (* (Math|Random|RandomUnitVectorinConeinDegrees (Math|Vector|GetUpVector (Variables|/Game/Blueprints/Gibs/BaseGibs_BP.BaseGibs_BP_C|GetBaseGibMesh _returnvalue_5)) 75.0) (Math|Random|RandomFloatinRange 5e+02 9e+02)) "None" true))
    (Game|SpawnActorfromClass "/Game/Blueprints/Auditory/EnemySoundActor_BP.EnemySoundActor_BP_C" (Math|Transform|MakeTransform (Transformation|GetWorldLocation (Variables|Default|GetSkeletalMeshREF)) "0, 0, 0" "1.000000,1.000000,1.000000") "Undefined" "MultiplyWithRoot" 0 9e+02 0)
    (Actor|DestroyActor)
    (else
      (for _index_2 (range 0 5)
        (bind _returnvalue_6 (Game|SpawnActorfromClass "/Game/Blueprints/Gibs/BaseGibs_BP.BaseGibs_BP_C" (Math|Transform|MakeTransform (Math|Vector|MakeVector (.x _returnvalue_3) 0.0 (.z _returnvalue_3)) (Math|Random|RandomRotator false) (Math|Vector|MakeVector _returnvalue _returnvalue _returnvalue)) "AlwaysSpawn" "MultiplyWithRoot" 0 0))
        (Components|StaticMesh|SetStaticMesh (Variables|/Game/Blueprints/Gibs/BaseGibs_BP.BaseGibs_BP_C|GetBaseGibMesh _returnvalue_6) (Variables|/Script/Engine.StaticMeshComponent|GetStaticMesh _staticmeshref_2))
        (Rendering|Material|SetMaterial (Variables|/Game/Blueprints/Gibs/BaseGibs_BP.BaseGibs_BP_C|GetBaseGibMesh _returnvalue_6) 0 (Rendering|Material|GetMaterial _staticmeshref_2 0))
        (Physics|AddImpulse (Variables|/Game/Blueprints/Gibs/BaseGibs_BP.BaseGibs_BP_C|GetBaseGibMesh _returnvalue_6) (* (Math|Random|RandomUnitVectorinConeinDegrees (Math|Vector|GetUpVector (Variables|/Game/Blueprints/Gibs/BaseGibs_BP.BaseGibs_BP_C|GetBaseGibMesh _returnvalue_6)) 75.0) (Math|Random|RandomFloatinRange 5e+02 9e+02)) "None" true))
      (Actor|DestroyActor))))

(event EventDisableGravity
  (bind _staticmeshref (Variables|Default|GetStaticMeshREF))
  (bind _skeletalmeshref (Variables|Default|GetSkeletalMeshREF))
  ;[0.15 0.15 0.15 0.5] Thrown State
  (if (== (Variables|Default|GetStaticMeshModel) 0)
    (Physics|SetEnableGravity _skeletalmeshref false)
    (Variables|Default|SetSkeletalMeshThrownVelocity (Transformation|GetComponentVelocity _skeletalmeshref))
    (else
      (Physics|SetEnableGravity _staticmeshref false)
      (Variables|Default|SetStaticMeshThrownVelocity (Transformation|GetComponentVelocity _staticmeshref)))))

(event EventBeginPlay
  ;[0.15 0.15 0.15 0.5] beginplay
  (Utilities|FlowControl|Sequence
    (:then_0
      ;[0.15 0.15 0.15 0.5] beginplay - check mesh validity
      (CallFunction|CheckMeshValidity))
    (:then_1
      ;[0.15 0.15 0.15 0.5] Store Player REF
      (bind _asbp_third_person_character (Utilities|Casting|CastToBP_ThirdPersonCharacter (Game|GetPlayerCharacter 0)))
      (Variables|Default|SetPlayerREF _asbp_third_person_character)
      (Actor|SetOwner _asbp_third_person_character))))

(event EventRequestPickUp
  (params (PlayerREF :type Actor%20Object%20Reference))
  ;[0.15 0.15 0.15 0.5] When player tries to interact with me, give player my REF and trigger event
  (Class|OLDInteractBPI|AddtoPlayer(Message) PlayerREF self (Variables|Default|GetStaticMeshREF) (Variables|Default|GetSkeletalMeshREF))
  (Rendering|SetVisibility (Variables|Default|GetGrabBilboard) false false))

(fn ConstructionScript
  ;[0.15 0.15 0.15 0.5] Assign Mesh on Cosntruction Script
  (Utilities|FlowControl|DoOnce false
    (:Completed
      (if (== (Variables|Default|GetStaticMeshModel) 0)
        (if (not (== (Variables|Default|GetSkeletalMeshModel) 0))
          (bind _returnvalue (AddComponent|AddSkeletalMeshComponent true (Math|Conversions|ToTransform(Vector) (Transformation|GetActorLocation))))
          (Transformation|AttachComponentToComponent _returnvalue (Variables|Default|GetDefaultSceneRoot) "None" "SnapToTarget" "SnapToTarget" "SnapToTarget" false)
          (Transformation|AttachComponentToComponent (Variables|Default|GetGrabBilboard) _returnvalue "None" "KeepRelative" "SnapToTarget" "KeepWorld" false)
          (Transformation|AttachComponentToComponent (Variables|Default|GetGrabRange) _returnvalue "None" "KeepRelative" "SnapToTarget" "KeepWorld" false)
          (Transformation|SetRelativeRotation _returnvalue (Variables|Default|GetRelativeSkeletalRotation) false false)
          (Components|SkeletalMesh|SetSkeletalMeshAsset _returnvalue (Variables|Default|GetSkeletalMeshModel))
          (bind _output_get (Variables|Default|SetSkeletalMeshREF _returnvalue))
          (Physics|SetSimulatePhysics _output_get true)
          (Rendering|Material|SetMaterial _output_get 0 "/Engine/EngineMaterials/EmissiveMeshMaterial.EmissiveMeshMaterial")
          (Rendering|Material|SetMaterial _output_get 1 "/Engine/EngineMaterials/EmissiveMeshMaterial.EmissiveMeshMaterial"))
        (else
          (bind _returnvalue_2 (AddComponent|AddStaticMeshComponent true (Math|Conversions|ToTransform(Vector) (Transformation|GetActorLocation))))
          (Transformation|AttachComponentToComponent _returnvalue_2 (Variables|Default|GetDefaultSceneRoot) "None" "SnapToTarget" "SnapToTarget" "SnapToTarget" false)
          (Transformation|AttachComponentToComponent (Variables|Default|GetGrabBilboard) _returnvalue_2 "Spine" "KeepRelative" "SnapToTarget" "KeepWorld" false)
          (Transformation|AttachComponentToComponent (Variables|Default|GetGrabRange) _returnvalue_2 "Spine" "KeepRelative" "SnapToTarget" "KeepWorld" false)
          (Components|StaticMesh|SetStaticMesh _returnvalue_2 (Variables|Default|GetStaticMeshModel))
          (Variables|Default|SetStaticMeshREF _returnvalue_2))))))

(fn CheckMeshValidity
  ;[0.15 0.15 0.15 0.5] Deletes actor if no mesh variable is set
  (Utilities|FlowControl|DoOnce false
    (:Completed
      (if (== (Variables|Default|GetStaticMeshModel) 0)
        (if (== (Variables|Default|GetSkeletalMeshModel) 0)
          (Development|PrintString (Utilities|String|Append (Utilities|GetDisplayName self) " INTERACTIBLE HAS NO MESH!") true true "(R=1.000000,G=0.013964,B=0.000000,A=1.000000)" 5.0)
          (Actor|DestroyActor))))))