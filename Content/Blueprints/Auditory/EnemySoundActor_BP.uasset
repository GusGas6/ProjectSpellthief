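; Short-lived sound event actor that scales its ellipse widget and shockwave VFX to its Radius, then destroys itself after a delay.
; On BeginPlay a sphere trace sends SoundHeardMessage to actors within that radius.
; The message carries the X and Z of the ground point found by a downward trace, falling back to the actor's location.
; It also passes any Staircase_BP found by a small sphere trace at the sound's origin.
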(event EventBeginPlay
  (bind _returnvalue (Transformation|GetActorLocation))
  (bind _returnvalue_2 (Transformation|GetActorLocation))
  (bind _returnvalue_3 (Transformation|GetActorLocation))
  (bind _soundelipsewidget (Variables|Default|GetSoundElipseWidget))
  (bind _shockwavevfx (Variables|Default|GetShockwaveVFX))
  (Transformation|SetWorldScale3D _soundelipsewidget (* (/ (Variables|Default|GetRadius) 545.0) (Transformation|GetWorldScale _soundelipsewidget)))
  (Transformation|SetWorldScale3D _shockwavevfx (* (/ (Variables|Default|GetRadius) 225.0) (Transformation|GetWorldScale _shockwavevfx)))
  (bind (_outhits _returnvalue_4) (Collision|MultiSphereTraceByChannel _returnvalue _returnvalue (Variables|Default|GetRadius) "TraceTypeQuery1" false (Utilities|Array|MakeArray self) "None" true "(R=1.000000,G=0.000000,B=0.000000,A=1.000000)" "(R=0.000000,G=1.000000,B=0.000000,A=1.000000)" 3.0))
  (if _returnvalue_4
    (for _array_element _outhits
      (bind (_outhit _returnvalue_5) (Collision|LineTraceByChannel _returnvalue_3 (- _returnvalue_3 (Math|Vector|MakeVector 0.0 0.0 (Variables|Default|GetRadius))) "TraceTypeQuery1" false 0 "None"))
      (if _returnvalue_5
        (Variables|Default|SetLocation (.ImpactPoint (Collision|BreakHitResult _outhit)))
        (else
          (Variables|Default|SetLocation _returnvalue_3)))
      (bind (_outhits_2 _returnvalue_6) (Collision|MultiSphereTraceByChannel _returnvalue_2 _returnvalue_2 5.0 "TraceTypeQuery1" false (Utilities|Array|MakeArray self) "None"))
      (if _returnvalue_6
        (for _array_element_2 _outhits_2
          (if (== (Utilities|GetClass (.HitActor (Collision|BreakHitResult _array_element_2))) "/Game/Blueprints/InteractSystem/Staircase_BP.Staircase_BP_C")
            (Variables|Default|SetNearest%20Stairs (.HitActor (Collision|BreakHitResult _array_element_2))))
          (Class|InteractBPI|SoundHeard(Message) (.HitActor (Collision|BreakHitResult _array_element)) (Math|Vector|MakeVector (.x (Variables|Default|GetLocation)) 0.0 (.z (Variables|Default|GetLocation))) (Variables|Default|GetNearest%20Stairs)))
        (else
          (Class|InteractBPI|SoundHeard(Message) (.HitActor (Collision|BreakHitResult _array_element)) (Math|Vector|MakeVector (.x (Variables|Default|GetLocation)) 0.0 (.z (Variables|Default|GetLocation))) (Variables|Default|GetNearest%20Stairs))))))
  (Utilities|FlowControl|Delay 3.0)
  (Actor|DestroyActor))

(fn ConstructionScript)