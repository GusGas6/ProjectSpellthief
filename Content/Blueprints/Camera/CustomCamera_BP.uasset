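; Side-scrolling camera actor that follows the player on X and/or Z and carries a layered Paper2D parallax background.
; Edge collision checks stop following on an axis when they overlap level boundary actors, and Tick resumes it once the player crosses the camera centre, gated by wide/tall level flags.
; Construction assigns layer sprites; BeginPlay creates dynamic materials with per-layer parallax multipliers, which Tick feeds the camera's X position.
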(event OnComponentBeginOverlap(CameraCollisionCheckBack)
  (params (OverlappedComponent :type Primitive%20Component%20Object%20Reference) (OtherActor :type Actor%20Object%20Reference) (OtherComp :type Primitive%20Component%20Object%20Reference) (OtherBodyIndex :type Integer) (bFromSweep :type Boolean) (SweepResult :type Hit%20Result%20Structure%20%28by%20ref%29))
  ;[0.15 0.15 0.15 0.5] Camera Control
  (if (== (Utilities|GetClass OtherActor) "/Game/Blueprints/LevelBoundarySide_BP.LevelBoundarySide_BP_C")
    (Variables|Default|SetInFrontOfCam false)
    (Variables|Default|SetStayOnPlayer false)
    (Utilities|FlowControl|DoOnce false) ; enters at Reset
  ))

(event OnComponentBeginOverlap(CameraCollisionCheckFront)
  (params (OverlappedComponent :type Primitive%20Component%20Object%20Reference) (OtherActor :type Actor%20Object%20Reference) (OtherComp :type Primitive%20Component%20Object%20Reference) (OtherBodyIndex :type Integer) (bFromSweep :type Boolean) (SweepResult :type Hit%20Result%20Structure%20%28by%20ref%29))
  ;[0.15 0.15 0.15 0.5] Camera Control
  (if (== (Utilities|GetClass OtherActor) "/Game/Blueprints/LevelBoundarySide_BP.LevelBoundarySide_BP_C")
    (Variables|Default|SetInFrontOfCam true)
    (Variables|Default|SetStayOnPlayer false)
    (Utilities|FlowControl|DoOnce false) ; enters at Reset
  ))

(event OnComponentBeginOverlap(CameraCollisionCheckTop)
  (params (OverlappedComponent :type Primitive%20Component%20Object%20Reference) (OtherActor :type Actor%20Object%20Reference) (OtherComp :type Primitive%20Component%20Object%20Reference) (OtherBodyIndex :type Integer) (bFromSweep :type Boolean) (SweepResult :type Hit%20Result%20Structure%20%28by%20ref%29))
  ;[0.15 0.15 0.15 0.5] Camera Control
  (if (== (Utilities|GetClass OtherActor) "/Game/Blueprints/LevelBoundaryTopBottom_BP.LevelBoundaryTopBottom_BP_C")
    (Variables|Default|SetAboveCam true)
    (Variables|Default|SetFollowUpAndDown false)
    (Variables|Default|SetStayOnPlayerVertical false)
    (Utilities|FlowControl|DoOnce false) ; enters at Reset
  ))

(event OnComponentBeginOverlap(CameraCollisionCheckBottom)
  (params (OverlappedComponent :type Primitive%20Component%20Object%20Reference) (OtherActor :type Actor%20Object%20Reference) (OtherComp :type Primitive%20Component%20Object%20Reference) (OtherBodyIndex :type Integer) (bFromSweep :type Boolean) (SweepResult :type Hit%20Result%20Structure%20%28by%20ref%29))
  ;[0.15 0.15 0.15 0.5] Camera Control
  (if (== (Utilities|GetClass OtherActor) "/Game/Blueprints/LevelBoundaryTopBottom_BP.LevelBoundaryTopBottom_BP_C")
    (Variables|Default|SetAboveCam false)
    (Variables|Default|SetFollowUpAndDown false)
    (Variables|Default|SetStayOnPlayerVertical false)
    (Utilities|FlowControl|DoOnce false) ; enters at Reset
  ))

(event EventTick
  (params (DeltaSeconds :type Float%20%28single-precision%29))
  (bind _returnvalue (Transformation|GetActorLocation))
  (bind _returnvalue_2 (Game|GetPlayerCharacter 0))
  (bind _returnvalue_3 (Transformation|GetActorLocation))
  (bind _returnvalue_4 (Transformation|GetActorLocation _returnvalue_2))
  ;[0.15 0.15 0.15 0.5] event tick
  ;[0.15 0.15 0.15 0.5] Camera Control
  (Utilities|FlowControl|Sequence
    (:then_0
      (Utilities|FlowControl|Sequence
        (:then_0
          (if (Variables|AllowCameraMovement|GetWIDE%20LEVEL)
            (if (Variables|Default|GetInFrontOfCam)
              (if (<= (.x (Transformation|GetActorLocation (Game|GetPlayerCharacter 0))) (.x (Transformation|GetActorLocation)))
                (Utilities|FlowControl|DoOnce false :!label _label
                  (:Completed
                    (Variables|Default|SetStayOnPlayer true))))
              (elif (>= (.x (Transformation|GetActorLocation (Game|GetPlayerCharacter 0))) (.x (Transformation|GetActorLocation)))
                (goto _label)))))
        (:then_1
          (if (Variables|AllowCameraMovement|GetTALL%20LEVEL)
            (if (Variables|Default|GetAboveCam)
              (if (<= (.z (Transformation|GetActorLocation (Game|GetPlayerCharacter 0))) (.z (Transformation|GetActorLocation)))
                (Utilities|FlowControl|DoOnce false :!label _label_2
                  (:Completed
                    (Variables|Default|SetStayOnPlayerVertical true)
                    (Variables|Default|SetFollowUpAndDown true))))
              (elif (>= (.z (Transformation|GetActorLocation (Game|GetPlayerCharacter 0))) (.z (Transformation|GetActorLocation)))
                (goto _label_2)))))))
    (:then_1
      (if (or (Variables|Default|GetStayOnPlayer) (Variables|Default|GetStayOnPlayerVertical))
        (if (Variables|Default|GetFollowUpAndDown)
          (if (Variables|Default|GetStayOnPlayer)
            (Transformation|SetActorLocation (Math|Vector|MakeVector (.x _returnvalue_4) (.y (Transformation|GetActorLocation)) (.z _returnvalue_4)) false false)
            (else
              (Transformation|SetActorLocation (Math|Vector|MakeVector (.x _returnvalue) (.y _returnvalue) (.z (Transformation|GetActorLocation (Game|GetPlayerCharacter 0)))) false false)))
          (else
            (Transformation|SetActorLocation (Math|Vector|MakeVector (.x (Transformation|GetActorLocation (Game|GetPlayerCharacter 0))) (.y _returnvalue_3) (.z _returnvalue_3)) false false)))))
    (:then_2
      ;[0.005089 0.08776 0.15 0.5] Set Camera Pos X (Parallax)
      (for _array_element (Variables|Default|GetDynamicLayers)
        (Rendering|Material|SetScalarParameterValue _array_element "CameraPosX" (.x (Transformation|GetWorldLocation (Variables|Default|GetCamera))) :!class /Script/Engine.MaterialInstanceDynamic)))))

(event EventBeginPlay
  ;[0.15 0.15 0.15 0.5] beginplay
  ;[7.5e-05 0.1297 0.15 0.5] Init Dynamic Material
  (for (_array_element _array_index) (Components|GetChildrenComponents (Variables|Default|GetStaticBackground) false)
    (bind _aspaper_sprite_component (Utilities|Casting|CastToPaperSpriteComponent _array_element))
    (bind _returnvalue (Rendering|Material|CreateDynamicMaterialInstance _aspaper_sprite_component 0 0 "None" :!class /Script/Engine.PrimitiveComponent))
    (Utilities|Array|Add (Variables|Default|GetDynamicLayers) _returnvalue)
    (Rendering|Material|SetScalarParameterValue _returnvalue "ParallaxMultiplier" (Utilities|Array|Get(acopy) (Variables|BackgroundSprites|GetParallaxMultipliers) _array_index) :!class /Script/Engine.MaterialInstanceDynamic)))

(fn ConstructionScript
  (Rendering|Components|Sprite|SetSprite (Variables|Default|GetStaticBackground) (Variables|BackgroundSprites|GetStaticBackgroundSprite))
  (Rendering|Components|Sprite|SetSprite (Variables|Default|Get4thLayer%28Translucent%29) (Variables|BackgroundSprites|Get4thLayerSprite%28Translucent%29))
  (Rendering|Components|Sprite|SetSprite (Variables|Default|Get5thLayer) (Variables|BackgroundSprites|Get5thLayerSprite))
  (Rendering|Components|Sprite|SetSprite (Variables|Default|Get3rdLayer) (Variables|BackgroundSprites|Get3rdLayerSprite))
  (Rendering|Components|Sprite|SetSprite (Variables|Default|Get2ndLayer) (Variables|BackgroundSprites|Get2ndLayerSprite)))