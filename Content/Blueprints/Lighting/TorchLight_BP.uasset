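; TorchLight_BP is a torch actor with a flickering point light and a particle effect.
; After a random start delay, it repeatedly picks one of three timelines at random to drive the light's intensity between a low and high value, looping when each finishes.
; A Bump event toggles the torch on or off by activating or deactivating the particles and showing or hiding the light.
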(event EventBeginPlay
  (Utilities|FlowControl|Delay (Math|Random|RandomFloatinRange 0.0 1.0))
  (switch int (Math|Random|RandomIntegerinRange 0 2) :!label _label
    (:0
      (bind _newtrack_0 (Timeline|Timeline PlayFromStart)
        (:Update
          (Rendering|Components|Light|SetIntensity (Variables|Default|GetPointLight) (Math|Float|Lerp 5e+02 2e+03 _newtrack_0)))
        (:Finished
          (Utilities|FlowControl|Sequence
            (:then_0
              (goto _label))))))
    (:1
      (bind _newtrack_0_2 (Timeline|Timeline_0 PlayFromStart)
        (:Update
          (Rendering|Components|Light|SetIntensity (Variables|Default|GetPointLight) (Math|Float|Lerp 5e+02 2e+03 _newtrack_0_2)))
        (:Finished
          (Utilities|FlowControl|Sequence
            (:then_0
              (goto _label))))))
    (:2
      (bind _newtrack_0_3 (Timeline|Timeline_1 PlayFromStart)
        (:Update
          (Rendering|Components|Light|SetIntensity (Variables|Default|GetPointLight) (Math|Float|Lerp 5e+02 2e+03 _newtrack_0_3)))
        (:Finished
          (Utilities|FlowControl|Sequence
            (:then_0
              (goto _label))))))))

(event EventBump
  (params (ON :type Boolean))
  (bind _particlesystem (Variables|Default|GetParticleSystem))
  (bind _pointlight (Variables|Default|GetPointLight))
  (if ON
    (Components|Activation|Activate _particlesystem true)
    (Rendering|SetVisibility _pointlight true false)
    (else
      (Components|Activation|Deactivate _particlesystem)
      (Rendering|SetVisibility _pointlight false false))))

(fn ConstructionScript)