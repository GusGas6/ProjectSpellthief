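; Master torch actor that toggles a group of torch lights and a light-blocker volume, starting on or off via StartOff.
; The construction script spawns torches as child actors from a transform array and extrudes a dynamic mesh box matching the collision box.
; Interact flips a "DIM" tag that drives blocker visibility and torch BumpMessage calls.
; Actors inside or crossing the box receive DimLightMessage to dim or restore, with leaving always sending a restore.
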(event OnComponentEndOverlap(LightBlockerCollision)
  (params (OverlappedComponent :type Primitive%20Component%20Object%20Reference) (OtherActor :type Actor%20Object%20Reference) (OtherComp :type Primitive%20Component%20Object%20Reference) (OtherBodyIndex :type Integer))
  ;[0.15 0.006972 0.03 0.5] funky shit
  (Class|InteractBPI|DimLight(Message) OtherActor true))

(event OnComponentBeginOverlap(LightBlockerCollision)
  (params (OverlappedComponent :type Primitive%20Component%20Object%20Reference) (OtherActor :type Actor%20Object%20Reference) (OtherComp :type Primitive%20Component%20Object%20Reference) (OtherBodyIndex :type Integer) (bFromSweep :type Boolean) (SweepResult :type Hit%20Result%20Structure%20%28by%20ref%29))
  (if (Utilities|Array|ContainsItem (Variables|Actor|GetTags) "DIM")
    (Class|InteractBPI|DimLight(Message) OtherActor false self (Components|GetOwner))
    (else
      (Class|InteractBPI|DimLight(Message) OtherActor true))))

(event Custom|UpdateLight
  (params (On :type Boolean))
  (bind _tags (Variables|Actor|GetTags))
  (bind _dynamiclightblocker (Variables|Default|GetDynamicLightBlocker))
  (if On
    (Rendering|SetVisibility _dynamiclightblocker false false)
    (Utilities|Array|RemoveItem _tags "DIM")
    (else
      (Rendering|SetVisibility _dynamiclightblocker true false)
      (Utilities|Array|Add _tags "DIM")))
  (for _array_element (Variables|Default|GetTorchLightArray)
    (Class|InteractBPI|Bump(Message) (Variables|/Script/Engine.ChildActorComponent|GetChildActor _array_element) On)))

(event EventBeginPlay
  (Utilities|FlowControl|Sequence
    (:then_0
      (if (Variables|Default|GetStartOff)
        (CallFunction|UpdateLight false)
        (else
          (CallFunction|UpdateLight true))))
    (:then_1
      (Components|Box|SetBoxExtent (Variables|Default|GetLightBlockerCollision) (Math|Vector|MakeVector (Variables|Default|GetWidth) (Variables|Default|GetYThickness) (Variables|Default|GetHeight)) true)
      (Transformation|SetRelativeTransform (Variables|Default|GetLightBlockerCollision) (Variables|Default|GetBoxOriginLocation) false false))))

(event EventInteract
  (bind _tags (Variables|Actor|GetTags))
  (bind _returnvalue (Utilities|Array|ContainsItem _tags "DIM"))
  (bind _returnvalue_2 (not _returnvalue))
  (if _returnvalue
    (Utilities|Array|RemoveItem _tags "DIM")
    (else
      (Utilities|Array|Add _tags "DIM")))
  (for _array_element (Collision|GetOverlappingActors (Variables|Default|GetLightBlockerCollision) 0 :!class /Script/Engine.PrimitiveComponent)
    (Class|InteractBPI|DimLight(Message) _array_element _returnvalue_2 self (Components|GetOwner)))
  (CallFunction|UpdateLight _returnvalue_2))

(fn ConstructionScript
  (bind _polygon_vertices (Variables|Default|GetPolygon%20Vertices))
  (bind _ythickness (Variables|Default|GetYThickness))
  (bind _torchlightarray (Variables|Default|GetTorchLightArray))
  (bind _torchamountandlocations (Variables|Default|GetTorchAmountAndLocations))
  (bind _width (Variables|Default|GetWidth))
  (bind _returnvalue (Utilities|Array|Length _torchamountandlocations))
  (bind _returnvalue_2 (* _width -1.0))
  (bind _returnvalue_3 (* _ythickness -1.0))
  (Utilities|FlowControl|Sequence
    (:then_0
      (if (Variables|Default|GetStartOff)
        (CallFunction|UpdateLight false)
        (else
          (CallFunction|UpdateLight true))))
    (:then_1
      (bind _returnvalue_4 (AddComponent|AddDynamicMeshComponent false))
      (bind _output_get (Variables|Default|SetDynamicLightBlocker _returnvalue_4))
      (bind _returnvalue_5 (DynamicMeshComponent|GetDynamicMesh _output_get))
      (Variables|Default|SetDynamicMesh _returnvalue_5)
      (Utilities|Array|SetArrayElem _polygon_vertices 0 (Math|Vector2D|MakeVector2D _width _ythickness))
      (Utilities|Array|SetArrayElem _polygon_vertices 1 (Math|Vector2D|MakeVector2D _returnvalue_2 _ythickness))
      (Utilities|Array|SetArrayElem _polygon_vertices 2 (Math|Vector2D|MakeVector2D _returnvalue_2 _returnvalue_3))
      (Utilities|Array|SetArrayElem _polygon_vertices 3 (Math|Vector2D|MakeVector2D _width _returnvalue_3))
      (Utilities|FlowControl|DoOnce false
        (:Completed
          (Class|GeometryScriptLibraryMeshPrimitiveFunctions|AppendSimpleExtrudePolygon (Variables|Default|GetDynamicMesh) (Utilities|Struct|MakeGeometryScriptPrimitiveOptions "PerFace" false "Uniform" 0) (Variables|Default|GetBoxOriginLocation) (Variables|Default|GetPolygon%20Vertices) (* (Variables|Default|GetHeight) 2.0) 0 true "Center" 0)
          (Components|Box|SetBoxExtent (Variables|Default|GetLightBlockerCollision) (Math|Vector|MakeVector (Variables|Default|GetWidth) (Variables|Default|GetYThickness) (Variables|Default|GetHeight)) false)
          (Transformation|SetRelativeTransform (Variables|Default|GetLightBlockerCollision) (Variables|Default|GetBoxOriginLocation) false false)
          (Rendering|Material|SetMaterial (Variables|Default|GetDynamicLightBlocker) 0 "/Game/Materials/LightBlocker_Mat.LightBlocker_Mat")
          (if (Variables|Default|GetStartOff)
            (Rendering|SetVisibility (Variables|Default|GetDynamicLightBlocker) true false)
            (else
              (Rendering|SetVisibility (Variables|Default|GetDynamicLightBlocker) false false))))))
    (:then_2
      (if (not (<= _returnvalue 0))
        (for _index (range 1 _returnvalue)
          (bind _returnvalue_6 (AddComponent|AddChildActorComponent false))
          (Utilities|Array|Add _torchlightarray _returnvalue_6)
          (Utilities|FlowControl|Sequence
            (:then_0
              (for (_array_element _array_index) _torchlightarray
                (Transformation|SetRelativeTransform _array_element (Utilities|Array|Get(acopy) (Variables|Default|GetTorchAmountAndLocations) _array_index) false false)))
            (:then_1
              (for _array_element_2 (Variables|Default|GetTorchLightArray)
                (Class|InteractBPI|Bump(Message) (Variables|/Script/Engine.ChildActorComponent|GetChildActor _array_element_2) (not (Variables|Default|GetStartOff)))))))))))