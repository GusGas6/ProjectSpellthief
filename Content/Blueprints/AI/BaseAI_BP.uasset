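; Base enemy AI character, configured by an EnemyTypeDA data asset, that roams, patrols or sleeps until it spots and attacks the player.
; PlayerSpotted switches to aggressive movement and a chase loop of AIMoveTo calls.
; Near attack range, it tracks the player with line-of-sight checks and an aim beam, then plays an attack montage, adding a projectile if ranged.
; Point damage or pickup replaces it with a BaseInteractible_BP, ragdolled when shot.
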(event OnComponentBeginOverlap(GrabRange)
  (params (OverlappedComponent :type Primitive%20Component%20Object%20Reference) (OtherActor :type Actor%20Object%20Reference) (OtherComp :type Primitive%20Component%20Object%20Reference) (OtherBodyIndex :type Integer) (bFromSweep :type Boolean) (SweepResult :type Hit%20Result%20Structure%20%28by%20ref%29))
  ;[0.15 0.15 0.15 0.5] Toggle Grab Icon
  (if (== OtherActor (Variables|CoreREFs|GetPlayerREF))
    (Development|SetHiddeninGame (Variables|Default|GetGrabBilboard) false false)))

(event OnComponentEndOverlap(GrabRange)
  (params (OverlappedComponent :type Primitive%20Component%20Object%20Reference) (OtherActor :type Actor%20Object%20Reference) (OtherComp :type Primitive%20Component%20Object%20Reference) (OtherBodyIndex :type Integer))
  ;[0.15 0.15 0.15 0.5] Toggle Grab Icon
  (if (== OtherActor (Variables|CoreREFs|GetPlayerREF))
    (Development|SetHiddeninGame (Variables|Default|GetGrabBilboard) true false)))

(event Custom|Attacking
  (bind _playerinlos (CallFunction|CheckPlayerLOS))
  (bind _targetindicatorbeam_bp (Variables|Temporary|GetTargetIndicatorBeam_BP))
  (bind _targetindicatorbeam_bp_2 (Variables|Temporary|GetTargetIndicatorBeam_BP))
  ;[0.15 0.15 0.15 0.5] Attacking
  (if (not (Variables|EnemyVars|GetAttackingPlayer))
    (Class|NavMovementInterface|StopActiveMovement (Variables|Character|GetCharacterMovement))
    (Variables|EnemyVars|SetAttackingPlayer true)
    (Variables|Temporary|SetNoMoreTargeting false)
    (CallFunction|RepeatRotateTowardsPlayer)
    (Utilities|FlowControl|Sequence
      (:then_0
        (if _playerinlos
          (Development|PrintString "AIMING..." true true "(R=1.000000,G=0.836337,B=0.000000,A=1.000000)")
          (Utilities|FlowControl|RetriggerableDelay (Variables|EnemyVars|GetAimingDuration))
          (if (Variables|EnemyVars|GetAttackingPlayer)
            (Utilities|FlowControl|Sequence
              (:then_0
                (Utilities|FlowControl|Sequence
                  (:then_0
                    (Utilities|FlowControl|RetriggerableDelay (Variables|EnemyVars|GetRecoveryDuration))
                    (CallFunction|EndAttack))
                  (:then_1
                    (Variables|Temporary|SetNoMoreTargeting true)
                    (Utilities|IsValid _targetindicatorbeam_bp
                      (:Is%20Valid
                        (Actor|DestroyActor _targetindicatorbeam_bp))))))
              (:then_1
                (Development|PrintString "FIRE!" true true "(R=0.039791,G=1.000000,B=0.000000,A=1.000000)")
                ;;[0.15 0.1456 0 0.5] FIRINGRAPH
                (|FiringGraph)))
            (else
              (CallFunction|EndAttack)))
          (else
            (CallFunction|EndAttack))))
      (:then_1
        (Utilities|FlowControl|DelayUntilNextTick :!label _label)
        (if (and _playerinlos (Variables|EnemyVars|GetAttackingPlayer))
          (if (not (Variables|Temporary|GetNoMoreTargeting))
            (CallFunction|AimIndicator)
            (goto _label))
          (else
            (Utilities|IsValid _targetindicatorbeam_bp_2
              (:Is%20Valid
                (Actor|DestroyActor _targetindicatorbeam_bp_2))
              (:Is%20Not%20Valid
                _))
            (CallFunction|EndAttack)))))))

(event Custom|RepeatRotateTowardsPlayer
  ;[0.15 0.15 0.15 0.5] Rotating Towards Player Repeatedly
  (if (Variables|EnemyVars|GetAttackingPlayer)
    (CallFunction|RotateatPlayer)
    (Utilities|FlowControl|DelayUntilNextTick)
    (CallFunction|RepeatRotateTowardsPlayer)))

(event EventPlayerSpotted
  (params (PlayerREF :type Actor%20Object%20Reference))
  ;[0.15 0.15 0.15 0.5] Player Spotted Event
  (if (not (or (Variables|EnemyVars|GetBlind) (Variables|EnemyVars|GetSleeping)))
    (Development|PrintString "PLAYER SPOTTED" true true "(R=0.051574,G=1.000000,B=0.000000,A=1.000000)")
    (Class|AIUtilityBPI|UpdateSightColor(Message) (Variables|CoreREFs|GetVisionConeREF) true)
    (Class|NavMovementInterface|StopActiveMovement (Variables|Character|GetCharacterMovement))
    (Variables|EnemyVars|SetChasingPlayer true)
    (CallFunction|PlayerSpottedUpdateEnemyVariables)
    (CallFunction|ChasePlayer)))

(event EventDestroyed
  (bind _targetindicatorbeam_bp (Variables|Temporary|GetTargetIndicatorBeam_BP))
  ;[0.15 0.15 0.15 0.5] Event Destroyed
  (Variables|Temporary|SetNoMoreTargeting true)
  (Utilities|IsValid _targetindicatorbeam_bp
    (:Is%20Valid
      (Actor|DestroyActor _targetindicatorbeam_bp))))

(event Game|Damage|EventPointDamage
  (params (Damage :type Float%20%28single-precision%29) (DamageType :type Damage%20Type%20Object%20Reference) (HitLocation :type Vector :default "0, 0, 0") (HitNormal :type Vector :default "0, 0, 0") (HitComponent :type Primitive%20Component%20Object%20Reference) (BoneName :type Name :default "None") (ShotFromDirection :type Vector :default "0, 0, 0") (InstigatedBy :type Controller%20Object%20Reference) (DamageCauser :type Actor%20Object%20Reference) (HitInfo :type Hit%20Result%20Structure%20%28by%20ref%29))
  (bind _returnvalue (* Damage ShotFromDirection 3e+04))
  ;[0.15 0.15 0.15 0.5] Event Damage
  (Utilities|FlowControl|DoOnce false
    (:Completed
      (Class|NavMovementInterface|StopActiveMovement (Variables|Character|GetCharacterMovement))
      (bind _returnvalue_2 (Game|SpawnActorfromClass "/Game/Blueprints/Throwables/BaseInteractible_BP.BaseInteractible_BP_C" (Transformation|GetActorTransform) "Undefined" "MultiplyWithRoot" 0 0 (Components|SkeletalMesh|GetSkeletalMeshAsset (Variables|Character|GetMesh)) (Variables|/Script/Engine.SceneComponent|GetRelativeRotation (Variables|Character|GetMesh)) 0))
      (Utilities|IsValid (Variables|/Game/Blueprints/Throwables/BaseInteractible_BP.BaseInteractible_BP_C|GetSkeletalMeshREF _returnvalue_2)
        (:Is%20Valid
          (Physics|SetSimulatePhysics (Variables|/Game/Blueprints/Throwables/BaseInteractible_BP.BaseInteractible_BP_C|GetSkeletalMeshREF _returnvalue_2) true)
          (Physics|AddImpulse (Variables|/Game/Blueprints/Throwables/BaseInteractible_BP.BaseInteractible_BP_C|GetSkeletalMeshREF _returnvalue_2) (Math|Vector|MakeVector (.x _returnvalue) (.y _returnvalue) 0.0) BoneName true))
        (:Is%20Not%20Valid
          _))
      (Utilities|FlowControl|DelayUntilNextTick)
      (Actor|DestroyActor))))

(event EventRequestPickUp
  (params (PlayerREF :type Actor%20Object%20Reference))
  ;[0.15 0.15 0.15 0.5] Pick Up
  (bind _returnvalue (Game|SpawnActorfromClass "/Game/Blueprints/Throwables/BaseInteractible_BP.BaseInteractible_BP_C" (Transformation|GetActorTransform) "Undefined" "MultiplyWithRoot" 0 0 (Components|SkeletalMesh|GetSkeletalMeshAsset (Variables|Character|GetMesh)) "0.000000,0.000000,0.000000" 0))
  (Class|InteractBPI|RequestPickUp(Message) _returnvalue PlayerREF)
  (Actor|DestroyActor))

(event EventBeginPlay
  (bind _enemytype_da (Variables|EnemyType|GetEnemyType_DA))
  (bind _charactermovement (Variables|Character|GetCharacterMovement))
  ;[0.15 0.15 0.15 0.5] Beginplay
  (Variables|RandomRoam|SetSpawnLocation (Transformation|GetActorLocation))
  (Utilities|FlowControl|Sequence
    (:then_0
      (Utilities|FlowControl|Sequence
        (:then_0
          ;[0.15 0.15 0.15 0.5] EnemyStates
          (Utilities|FlowControl|DelayUntilNextTick)
          (CallFunction|SetEnemyStates))
        (:then_1
          ;[0.15 0.15 0.15 0.5] EnemyVariablesSet
          (CallFunction|SetEnemyTypeVars)
          (Utilities|FlowControl|DelayUntilNextTick)
          ;[0.15 0.15 0.15 0.5] Set Base Movespeed Variables
          (Variables|/Script/Engine.CharacterMovementComponent|SetMaxWalkSpeed _charactermovement (Variables|EnemyVars|GetBaseWalkSpeed))
          (Variables|/Script/Engine.CharacterMovementComponent|SetMaxAcceleration _charactermovement (Variables|EnemyVars|GetBaseMaxAcceleration))
          (Variables|/Script/Engine.CharacterMovementComponent|SetGroundFriction _charactermovement (Variables|EnemyVars|GetBaseGroundFriction))
          (Variables|/Game/Blueprints/Vision/VisionCone_BP.VisionCone_BP_C|SetVisionLength (Variables|CoreREFs|GetVisionConeREF) (Variables|/Game/Blueprints/DataAssets/Enemies/EnemyType_DA.EnemyType_DA_C|GetVisionLength _enemytype_da))
          (Variables|/Game/Blueprints/Vision/VisionCone_BP.VisionCone_BP_C|SetVisionArc (Variables|CoreREFs|GetVisionConeREF) (Variables|/Game/Blueprints/DataAssets/Enemies/EnemyType_DA.EnemyType_DA_C|GetVisionArc _enemytype_da)))))
    (:then_1
      ;[0.15 0.15 0.15 0.5] Set player REF
      (bind _asbp_player_character (Utilities|Casting|CastToBP_PlayerCharacter (Game|GetPlayerCharacter 0)))
      (bind _output_get (Variables|CoreREFs|SetPlayerREF _asbp_player_character))
      (Components|Sphere|SetSphereRadius (Variables|Default|GetGrabRange) (Variables|/Game/Blueprints/BP_PlayerCharacter.BP_PlayerCharacter_C|GetPickUpRange _output_get) true))
    (:then_2
      ;[0.15 0.15 0.15 0.5] Set Vision Cone REF
      (bind _asvision_cone_bp (Utilities|Casting|CastToVisionCone_BP (Variables|/Script/Engine.ChildActorComponent|GetChildActor (Variables|Default|GetVisionConeChildBP))))
      (Variables|CoreREFs|SetVisionConeREF _asvision_cone_bp))))

(fn ConstructionScript
  (Actor|SetOwner (Variables|/Script/Engine.ChildActorComponent|GetChildActor (Variables|Default|GetVisionConeChildBP)) self))

(fn CheckPlayerLOS
  (bind (_outhit _returnvalue) (Collision|LineTraceByChannel (.location (Transformation|GetBoneTransform (Variables|Character|GetMesh) "Head" "RTS_World")) (.location (Transformation|GetBoneTransform (Variables|/Script/Engine.Character|GetMesh (Variables|CoreREFs|GetPlayerREF)) "Head" "RTS_World")) "TraceTypeQuery2" false 0 "None"))
  (if _returnvalue
    (if (or (== (Variables|CoreREFs|GetPlayerREF) (.HitActor (Collision|BreakHitResult _outhit))) (== (.HitComponent (Collision|BreakHitResult _outhit)) (Variables|/Script/Engine.Character|GetMesh (Variables|CoreREFs|GetPlayerREF))))
      (return true)
      (else
        _)))
  (return false))

(fn RotateatPlayer
  (bind _returnvalue (Transformation|GetActorRotation))
  (Transformation|SetActorRotation (Math|Rotator|MakeRotator (.roll _returnvalue) (.pitch _returnvalue) (.yaw (Math|Conversions|RotationFromXVector (Math|Vector|GetUnitDirection(Vector) (Transformation|GetActorLocation) (Transformation|GetWorldLocation (Variables|/Script/Engine.Character|GetMesh (Variables|CoreREFs|GetPlayerREF)))))))))

(fn EndAttack
  (Variables|EnemyVars|SetAttackingPlayer false)
  (CallFunction|ChasePlayer))

(fn PlayerSpottedUpdateEnemyVariables
  (bind _charactermovement (Variables|Character|GetCharacterMovement))
  (bind _visionconeref (Variables|CoreREFs|GetVisionConeREF))
  (Utilities|FlowControl|DoOnce false
    (:Completed
      (Variables|/Script/Engine.CharacterMovementComponent|SetMaxWalkSpeed _charactermovement (Variables|EnemyVars|GetAggressiveWalkSpeed))
      (Variables|/Script/Engine.CharacterMovementComponent|SetMaxAcceleration _charactermovement (Variables|EnemyVars|GetAggressiveMaxAcceleration))
      (Variables|/Script/Engine.CharacterMovementComponent|SetGroundFriction _charactermovement (Variables|EnemyVars|GetAggressiveGroundFriction))
      (Variables|/Game/Blueprints/Vision/VisionCone_BP.VisionCone_BP_C|SetVisionLength _visionconeref (* (Variables|EnemyVars|GetAttackRange) 2.0))
      (Variables|/Game/Blueprints/Vision/VisionCone_BP.VisionCone_BP_C|SetVisionArc _visionconeref (* (Variables|/Game/Blueprints/Vision/VisionCone_BP.VisionCone_BP_C|GetVisionArc _visionconeref) 0.66)))))

(fn SetEnemyTypeVars
  (bind _enemytype_da (Variables|EnemyType|GetEnemyType_DA))
  (bind _enemytype_da_2 (Variables|EnemyType|GetEnemyType_DA))
  (bind _enemytype_da_3 (Variables|EnemyType|GetEnemyType_DA))
  (bind _enemytype_da_4 (Variables|EnemyType|GetEnemyType_DA))
  (bind _enemytype_da_5 (Variables|EnemyType|GetEnemyType_DA))
  (bind _enemytype_da_6 (Variables|EnemyType|GetEnemyType_DA))
  (Variables|EnemyVars|SetAttackRange (Variables|/Game/Blueprints/DataAssets/Enemies/EnemyType_DA.EnemyType_DA_C|GetAttackRange _enemytype_da_4))
  (Variables|EnemyVars|SetAttackRangeErrorTolerance (Variables|/Game/Blueprints/DataAssets/Enemies/EnemyType_DA.EnemyType_DA_C|GetAttackRangeErrorTolerance _enemytype_da_4))
  (Variables|EnemyVars|SetAimingDuration (Variables|/Game/Blueprints/DataAssets/Enemies/EnemyType_DA.EnemyType_DA_C|GetAimingDuration _enemytype_da_5))
  (Variables|EnemyVars|SetRecoveryDuration (Variables|/Game/Blueprints/DataAssets/Enemies/EnemyType_DA.EnemyType_DA_C|GetRecoveryDuration _enemytype_da_5))
  (Variables|EnemyVars|SetBaseWalkSpeed (Variables|/Game/Blueprints/DataAssets/Enemies/EnemyType_DA.EnemyType_DA_C|GetBaseWalkSpeed _enemytype_da))
  (Variables|EnemyVars|SetBaseMaxAcceleration (Variables|/Game/Blueprints/DataAssets/Enemies/EnemyType_DA.EnemyType_DA_C|GetBase%20Max%20Acceleration _enemytype_da))
  (Variables|EnemyVars|SetBaseGroundFriction (Variables|/Game/Blueprints/DataAssets/Enemies/EnemyType_DA.EnemyType_DA_C|GetBaseGroundFriction _enemytype_da))
  (Variables|EnemyVars|SetAggressiveWalkSpeed (Variables|/Game/Blueprints/DataAssets/Enemies/EnemyType_DA.EnemyType_DA_C|GetAggressiveWalkSpeed _enemytype_da_2))
  (Variables|EnemyVars|SetAggressiveMaxAcceleration (Variables|/Game/Blueprints/DataAssets/Enemies/EnemyType_DA.EnemyType_DA_C|GetAggressiveMaxAcceleration _enemytype_da_2))
  (Variables|EnemyVars|SetAggressiveGroundFriction (Variables|/Game/Blueprints/DataAssets/Enemies/EnemyType_DA.EnemyType_DA_C|GetAggressiveGroundFriction _enemytype_da_2))
  (Variables|EnemyVars|SetTimeBetweenAttacksFired (Variables|/Game/Blueprints/DataAssets/Enemies/EnemyType_DA.EnemyType_DA_C|GetTimeBetweenAttacksFired _enemytype_da_3))
  (Variables|EnemyVars|SetAttacksFiredPerAttack (Variables|/Game/Blueprints/DataAssets/Enemies/EnemyType_DA.EnemyType_DA_C|GetAttacksFiredPerAttack _enemytype_da_3))
  (Variables|EnemyVars|SetAimingAnimation (Variables|/Game/Blueprints/DataAssets/Enemies/EnemyType_DA.EnemyType_DA_C|GetAimingAnimation _enemytype_da_6))
  (Variables|EnemyVars|SetAttackAnimation (Variables|/Game/Blueprints/DataAssets/Enemies/EnemyType_DA.EnemyType_DA_C|GetAttackAnimation _enemytype_da_6))
  (Variables|EnemyVars|SetProjectile%20Type (Variables|/Game/Blueprints/DataAssets/Enemies/EnemyType_DA.EnemyType_DA_C|GetProjectileType _enemytype_da_6)))

(fn SetEnemyStates
  (switch Utilities|FlowControl|Switch|SwitchonEnemyStates_Enum (Variables|EnemyState|GetEnemyStatesEnum)
    (:NewEnumerator1
      (CallFunction|RandomRoam))
    (:NewEnumerator2
      (CallFunction|Patrolling))
    (:NewEnumerator3
      (CallFunction|ChasePlayer))
    (:NewEnumerator4
      (ChildActorComponent|SetChildActorClass (Variables|Default|GetVisionConeChildBP) 0)
      (Variables|EnemyVars|SetSleeping true))))

(fn AimIndicator
  (bind _bulletspawnloc (Variables|Default|GetBulletSpawnLoc))
  (bind _playerref (Variables|CoreREFs|GetPlayerREF))
  (bind _returnvalue (Transformation|GetWorldLocation _bulletspawnloc))
  (bind _mesh (Variables|/Script/Engine.Character|GetMesh _playerref))
  (bind _returnvalue_2 (Transformation|GetBoneTransform _mesh "Head" "RTS_World"))
  (Utilities|IsValid (Variables|Temporary|GetTargetIndicatorBeam_BP)
    (:Is%20Valid
      _)
    (:Is%20Not%20Valid
      (bind _returnvalue_3 (Game|SpawnActorfromClass "/Game/Spells/Beam/TargetIndicatorBeamActor_BP.TargetIndicatorBeamActor_BP_C" (Math|Transform|MakeTransform (Transformation|GetWorldLocation (Variables|Default|GetBulletSpawnLoc)) "0, 0, 0" "1.000000,1.000000,1.000000") "Undefined" "MultiplyWithRoot" 0 "1.000000,1.000000,1.000000" 0))
      (Variables|Temporary|SetTargetIndicatorBeam_BP _returnvalue_3)))
  (Utilities|IsValid (Variables|Temporary|GetTargetIndicatorBeam_BP)
    (:Is%20Valid
      (Class|ParticleSystemComponent|SetBeamSourcePoint (Variables|/Game/Spells/Beam/TargetIndicatorBeamActor_BP.TargetIndicatorBeamActor_BP_C|GetArcaneBeam (Variables|Temporary|GetTargetIndicatorBeam_BP)) 0 _returnvalue)
      (bind (_outhit _returnvalue_4) (Collision|LineTraceByChannel _returnvalue (.location _returnvalue_2) "TraceTypeQuery1" false 0 "None"))
      (if _returnvalue_4
        (if (== (.HitActor (Collision|BreakHitResult _outhit)) (Variables|/Script/Engine.Character|GetMesh _playerref))
          (Variables|Temporary|SetBeamEndLocation (.location _returnvalue_2) :!label _label)
          (else
            (Variables|Temporary|SetBeamEndLocation (.Location (Collision|BreakHitResult _outhit)))))
        (else
          (goto _label)))
      (Class|ParticleSystemComponent|SetBeamEndPoint (Variables|/Game/Spells/Beam/TargetIndicatorBeamActor_BP.TargetIndicatorBeamActor_BP_C|GetArcaneBeam (Variables|Temporary|GetTargetIndicatorBeam_BP)) 0 (Variables|Temporary|GetBeamEndLocation)))))

(event Custom|RandomRoam
  ;[0.15 0.15 0.15 0.5] Random Roam
  (if (not (Variables|EnemyVars|GetChasingPlayer))
    (AI|AIMoveTo self (.RandomLocation (AI|Navigation|GetRandomReachablePointinRadius (Variables|RandomRoam|GetSpawnLocation) (Variables|RandomRoam|GetRandomRoamRadius) 0 0)) 0 25.0 false
      (:OnSuccess
        _)
      (:OnFail
        _))
    (Utilities|FlowControl|Delay (Variables|Patrolling|GetWaitTimeBetweenPatrols))
    (Utilities|FlowControl|DelayUntilNextTick)
    (CallFunction|RandomRoam)))

(event Custom|Patrolling
  ;[0.15 0.15 0.15 0.5] Patrolling
  (if (not (Variables|EnemyVars|GetChasingPlayer))
    (AI|AIMoveTo self (.RandomLocation (AI|Navigation|GetRandomReachablePointinRadius (Transformation|GetActorLocation (Utilities|Array|Get(acopy) (Variables|Patrolling|GetPatrolPoints) (Variables|Patrolling|GetPatrolIndex))) 25.0 0 0)) 0 25.0 false
      (:OnSuccess
        _)
      (:OnFail
        _))
    (Utilities|FlowControl|Delay (Variables|Patrolling|GetWaitTimeBetweenPatrols))
    (Math|Integer|IncrementInt (Variables|Patrolling|GetPatrolIndex)
      (:%20%20
        (Utilities|FlowControl|DelayUntilNextTick)
        (if (>= (Variables|Patrolling|GetPatrolIndex) (Utilities|Array|Length (Variables|Patrolling|GetPatrolPoints)))
          (Variables|Patrolling|SetPatrolIndex 0))
        (CallFunction|Patrolling)))))

(event Custom|Chase%20Player
  (bind _playerref (Variables|CoreREFs|GetPlayerREF))
  ;[0.15 0.15 0.15 0.5] Chase Player
  (Utilities|IsValid _playerref
    (:Is%20Valid
      (AI|AIMoveTo self (.RandomLocation (AI|Navigation|GetRandomReachablePointinRadius (Transformation|GetWorldLocation (Variables|/Script/Engine.Character|GetMesh _playerref)) 25.0 0 0)) 0 25.0 false
        (:then
          (Utilities|FlowControl|DelayUntilNextTick)
          (if (Math|Float|NearlyEqual(Float) (Math|Vector|Distance(Vector) (Transformation|GetWorldLocation (Variables|/Script/Engine.Character|GetMesh (Variables|CoreREFs|GetPlayerREF))) (Transformation|GetActorLocation)) (Variables|EnemyVars|GetAttackRange) (Variables|EnemyVars|GetAttackRangeErrorTolerance))
            (CallFunction|Attacking)
            (else
              (CallFunction|ChasePlayer))))))))