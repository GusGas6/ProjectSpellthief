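; Staircase door actor that links to optional up and down staircases and animates characters entering and exiting.
; Overlap volumes register it as actors' nearest stairs, while player proximity also sends the linked stairs and swings the door open.
; Use and exit events message the moving actor, then chained timelines animate the door and a DoorPersonHere anchor, with BeingUsed delaying closure.
; It also shows a cursor tooltip and loops a light-intensity animation.
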(event OnComponentBeginOverlap(Box)
  (params (OverlappedComponent :type Primitive%20Component%20Object%20Reference) (OtherActor :type Actor%20Object%20Reference) (OtherComp :type Primitive%20Component%20Object%20Reference) (OtherBodyIndex :type Integer) (bFromSweep :type Boolean) (SweepResult :type Hit%20Result%20Structure%20%28by%20ref%29))
  (bind _returnvalue (Game|GetPlayerCharacter 0))
  (bind _upstairscase (Variables|Default|GetUpStairscase))
  (bind _downstaircase (Variables|Default|GetDownStaircase))
  (if (== (Game|GetPlayerCharacter 0) OtherActor)
    (Utilities|FlowControl|DelayUntilNextTick)
    (Utilities|FlowControl|Sequence
      (:then_0
        (Utilities|IsValid _upstairscase
          (:Is%20Valid
            (Class|InteractBPI|Staircase(Message) _returnvalue _upstairscase _downstaircase)
            (Class|InteractBPI|SetNearestStairs(Message) _returnvalue self :!label _label))))
      (:then_1
        (Utilities|IsValid _downstaircase
          (:Is%20Valid
            (Class|InteractBPI|Staircase(Message) _returnvalue _upstairscase _downstaircase)
            (goto _label))))
      (:then_2
        (bind _newtrack_0 (Timeline|Timeline Play)
          (:Update
            (Transformation|SetRelativeRotation (Variables|Default|GetDoorMesh) (Math|Rotator|Lerp(Rotator) "0, 0, 0" "0.000000,-40.000000,0.000000" _newtrack_0) false false)))))))

(event OnComponentEndOverlap(Box)
  (params (OverlappedComponent :type Primitive%20Component%20Object%20Reference) (OtherActor :type Actor%20Object%20Reference) (OtherComp :type Primitive%20Component%20Object%20Reference) (OtherBodyIndex :type Integer))
  (if (== (Game|GetPlayerCharacter 0) OtherActor)
    (Class|InteractBPI|Staircase(Message) (Game|GetPlayerCharacter 0))
    (Utilities|FlowControl|Sequence
      (:then_0
        (bind _newtrack_0 (Timeline|Timeline Stop)
          (:Update
            (Transformation|SetRelativeRotation (Variables|Default|GetDoorMesh) (Math|Rotator|Lerp(Rotator) "0, 0, 0" "0.000000,-40.000000,0.000000" _newtrack_0) false false))))
      (:then_1
        (Utilities|FlowControl|DelayUntilNextTick)
        (if (not (Variables|Default|GetBeingUsed))
          (Timeline|Timeline Reverse))))))

(event OnComponentBeginOverlap(NearestStairBox)
  (params (OverlappedComponent :type Primitive%20Component%20Object%20Reference) (OtherActor :type Actor%20Object%20Reference) (OtherComp :type Primitive%20Component%20Object%20Reference) (OtherBodyIndex :type Integer) (bFromSweep :type Boolean) (SweepResult :type Hit%20Result%20Structure%20%28by%20ref%29))
  ;[0.15 0.15 0.15 0.5] Set Nearest Stairs
  (Class|InteractBPI|SetNearestStairs(Message) OtherActor self))

(event Custom|PersonExitsDoor
  (params (ActorToMove :type Actor%20Object%20Reference))
  (bind _doorpersonhere (Variables|Default|GetDoorPersonHere))
  (bind _doorpersonhere_2 (Variables|Default|GetDoorPersonHere))
  (Class|InteractBPI|ExitStairs(Message) ActorToMove self (Variables|Default|GetDoorPersonHere))
  (Variables|Default|SetBeingUsed true)
  (Utilities|FlowControl|Sequence
    (:then_0
      (CallFunction|StopAllDoorAnims)
      (Utilities|FlowControl|Sequence
        (:then_0
          (bind _newtrack_0 (Timeline|Timeline_4 PlayFromStart)
            (:Update
              (Transformation|SetRelativeLocation _doorpersonhere_2 (Math|Vector|Lerp(Vector) "30.000000,-300.000000,0.000000" "30.000000,-200.000000,0.000000" _newtrack_0) false false)
              (Transformation|SetRelativeRotation (Variables|Default|GetDoorMesh) (Math|Rotator|Lerp(Rotator) "0.000000,-40.000000,0.000000" "0.000000,-60.000000,0.000000" _newtrack_0) false false))))
        (:then_1
          (bind _newtrack_0_2 (Timeline|Timeline_5 PlayFromStart)
            (:Update
              (Transformation|SetRelativeRotation _doorpersonhere_2 (Math|Rotator|Lerp(Rotator) "0.000000,0.000000,0.000000" "0.000000,-180.000000,0.000000" _newtrack_0_2) false false))
            (:Finished
              (Utilities|FlowControl|Sequence
                (:then_0
                  (bind _newtrack_0_3 (Timeline|Timeline_6 PlayFromStart)
                    (:Update
                      (Transformation|SetRelativeLocation _doorpersonhere (Math|Vector|Lerp(Vector) "30.000000,-200.000000,0.000000" "0.000000,0.000000,0.000000" _newtrack_0_3) false false)
                      (Transformation|SetRelativeRotation (Variables|Default|GetDoorMesh) (Math|Rotator|Lerp(Rotator) "0.000000,-60.000000,0.000000" "0.000000,-40.000000,0.000000" _newtrack_0_3) false false))))
                (:then_1
                  (bind _newtrack_0_4 (Timeline|Timeline_7 PlayFromStart)
                    (:Update
                      (Transformation|SetRelativeRotation _doorpersonhere (Math|Rotator|Lerp(Rotator) "0.000000,-180.000000,0.000000" "0.000000,0.000000,0.000000" _newtrack_0_4 true) false false))))))))))
    (:then_1
      (Utilities|FlowControl|RetriggerableDelay 0.5)
      (Variables|Default|SetBeingUsed false))))

(event Custom|StopAllDoorAnims
  (bind _doorpersonhere (Variables|Default|GetDoorPersonHere))
  (bind _doorpersonhere_2 (Variables|Default|GetDoorPersonHere))
  (bind _doorpersonhere_3 (Variables|Default|GetDoorPersonHere))
  (bind _doorpersonhere_4 (Variables|Default|GetDoorPersonHere))
  (Utilities|FlowControl|Sequence
    (:then_0
      (bind _newtrack_0 (Timeline|Timeline Stop)
        (:Update
          (Transformation|SetRelativeRotation (Variables|Default|GetDoorMesh) (Math|Rotator|Lerp(Rotator) "0, 0, 0" "0.000000,-40.000000,0.000000" _newtrack_0) false false))))
    (:then_1
      (bind _newtrack_0_2 (Timeline|Timeline_1 Stop)
        (:Update
          (Transformation|SetRelativeLocation _doorpersonhere (Math|Vector|Lerp(Vector) "30.000000,-106.000000,0.000000" "30.000000,-300.000000,0.000000" _newtrack_0_2) false false)
          (Transformation|SetRelativeRotation (Variables|Default|GetDoorMesh) (Math|Rotator|Lerp(Rotator) "0.000000,-40.000000,0.000000" "0.000000,-60.000000,0.000000" _newtrack_0_2) false false))))
    (:then_2
      (bind _newtrack_0_3 (Timeline|s Stop)
        (:Update
          (Transformation|SetRelativeRotation _doorpersonhere (Math|Rotator|Lerp(Rotator) "0.000000,-180.000000,0.000000" "0.000000,-280.000000,0.000000" _newtrack_0_3) false false))
        (:Finished
          (Utilities|FlowControl|Sequence
            (:then_0
              (bind _newtrack_0_4 (Timeline|Timeline_2 PlayFromStart)
                (:Update
                  (Transformation|SetRelativeLocation _doorpersonhere_2 (Math|Vector|Lerp(Vector) "30.000000,-300.000000,0.000000" "30.000000,-210.000000,0.000000" _newtrack_0_4) false false)
                  (Transformation|SetRelativeRotation (Variables|Default|GetDoorMesh) (Math|Rotator|Lerp(Rotator) "0.000000,-60.000000,0.000000" "0.000000,0.000000,0.000000" _newtrack_0_4) false false))))
            (:then_1
              (bind _newtrack_0_5 (Timeline|Timeline_3 PlayFromStart)
                (:Update
                  (Transformation|SetRelativeRotation _doorpersonhere_2 (Math|Rotator|Lerp(Rotator) "0.000000,-280.000000,0.000000" "0.000000,-400.000000,0.000000" _newtrack_0_5 true) false false))))))))
    (:then_3
      (Timeline|Timeline_2 Stop))
    (:then_4
      (Timeline|Timeline_3 Stop))
    (:then_5
      (bind _newtrack_0_6 (Timeline|Timeline_4 Stop)
        (:Update
          (Transformation|SetRelativeLocation _doorpersonhere_4 (Math|Vector|Lerp(Vector) "30.000000,-300.000000,0.000000" "30.000000,-200.000000,0.000000" _newtrack_0_6) false false)
          (Transformation|SetRelativeRotation (Variables|Default|GetDoorMesh) (Math|Rotator|Lerp(Rotator) "0.000000,-40.000000,0.000000" "0.000000,-60.000000,0.000000" _newtrack_0_6) false false))))
    (:then_6
      (bind _newtrack_0_7 (Timeline|Timeline_5 Stop)
        (:Update
          (Transformation|SetRelativeRotation _doorpersonhere_4 (Math|Rotator|Lerp(Rotator) "0.000000,0.000000,0.000000" "0.000000,-180.000000,0.000000" _newtrack_0_7) false false))
        (:Finished
          (Utilities|FlowControl|Sequence
            (:then_0
              (bind _newtrack_0_8 (Timeline|Timeline_6 PlayFromStart)
                (:Update
                  (Transformation|SetRelativeLocation _doorpersonhere_3 (Math|Vector|Lerp(Vector) "30.000000,-200.000000,0.000000" "0.000000,0.000000,0.000000" _newtrack_0_8) false false)
                  (Transformation|SetRelativeRotation (Variables|Default|GetDoorMesh) (Math|Rotator|Lerp(Rotator) "0.000000,-60.000000,0.000000" "0.000000,-40.000000,0.000000" _newtrack_0_8) false false))))
            (:then_1
              (bind _newtrack_0_9 (Timeline|Timeline_7 PlayFromStart)
                (:Update
                  (Transformation|SetRelativeRotation _doorpersonhere_3 (Math|Rotator|Lerp(Rotator) "0.000000,-180.000000,0.000000" "0.000000,0.000000,0.000000" _newtrack_0_9 true) false false))))))))
    (:then_7
      (Timeline|Timeline_6 Stop))
    (:then_8
      (Timeline|Timeline_7 Stop))))

(event Custom|PersonEntersDoor
  (params (ActorToMove :type Actor%20Object%20Reference))
  (bind _doorpersonhere (Variables|Default|GetDoorPersonHere))
  (bind _doorpersonhere_2 (Variables|Default|GetDoorPersonHere))
  (Class|InteractBPI|UseStairs(Message) ActorToMove self (Variables|Default|GetDoorPersonHere))
  (CallFunction|StopAllDoorAnims)
  (Variables|Default|SetBeingUsed true)
  (Utilities|FlowControl|Sequence
    (:then_0
      (bind _newtrack_0 (Timeline|Timeline_1 PlayFromStart)
        (:Update
          (Transformation|SetRelativeLocation _doorpersonhere (Math|Vector|Lerp(Vector) "30.000000,-106.000000,0.000000" "30.000000,-300.000000,0.000000" _newtrack_0) false false)
          (Transformation|SetRelativeRotation (Variables|Default|GetDoorMesh) (Math|Rotator|Lerp(Rotator) "0.000000,-40.000000,0.000000" "0.000000,-60.000000,0.000000" _newtrack_0) false false))))
    (:then_1
      (bind _newtrack_0_2 (Timeline|s PlayFromStart)
        (:Update
          (Transformation|SetRelativeRotation _doorpersonhere (Math|Rotator|Lerp(Rotator) "0.000000,-180.000000,0.000000" "0.000000,-280.000000,0.000000" _newtrack_0_2) false false))
        (:Finished
          (Utilities|FlowControl|Sequence
            (:then_0
              (bind _newtrack_0_3 (Timeline|Timeline_2 PlayFromStart)
                (:Update
                  (Transformation|SetRelativeLocation _doorpersonhere_2 (Math|Vector|Lerp(Vector) "30.000000,-300.000000,0.000000" "30.000000,-210.000000,0.000000" _newtrack_0_3) false false)
                  (Transformation|SetRelativeRotation (Variables|Default|GetDoorMesh) (Math|Rotator|Lerp(Rotator) "0.000000,-60.000000,0.000000" "0.000000,0.000000,0.000000" _newtrack_0_3) false false))))
            (:then_1
              (bind _newtrack_0_4 (Timeline|Timeline_3 PlayFromStart)
                (:Update
                  (Transformation|SetRelativeRotation _doorpersonhere_2 (Math|Rotator|Lerp(Rotator) "0.000000,-280.000000,0.000000" "0.000000,-400.000000,0.000000" _newtrack_0_4 true) false false))))))))
    (:then_2
      (Utilities|FlowControl|RetriggerableDelay 0.5)
      (Variables|Default|SetBeingUsed false))))

(event EventBeginPlay
  (Utilities|FlowControl|Sequence
    (:then_0
      (Utilities|FlowControl|DelayUntilNextTick)
      (for _array_element (Collision|GetOverlappingActors (Variables|Default|GetNearestStairBox) 0 :!class /Script/Engine.PrimitiveComponent)
        (Class|InteractBPI|SetNearestStairs(Message) _array_element self)))
    (:then_1
      (bind _newtrack_0 (Timeline|Timeline_0 PlayFromStart)
        (:Update
          (Rendering|Components|Light|SetIntensity (Variables|Default|GetPointLight) (Math|Float|Lerp 1e+03 4e+03 _newtrack_0)))
        (:Finished
          (Utilities|FlowControl|Sequence
            (:then_0
              (Timeline|Timeline_0 PlayFromStart))))))))

(event EventUseStairs
  (params (ActorRef :type Actor%20Object%20Reference) (PersonLocRef :type Skeletal%20Mesh%20Component%20Object%20Reference))
  (CallFunction|PersonEntersDoor ActorRef))

(event EventExitStairs
  (params (ActorRef :type Actor%20Object%20Reference) (PersonLocRef :type Skeletal%20Mesh%20Component%20Object%20Reference))
  (CallFunction|PersonExitsDoor ActorRef))

(event MouseInput|EventActorBeginCursorOver
  ;[0.15 0.15 0.15 0.5] Tooltip
  (Class|InteractBPI|SetToolTip(Message) (Game|GetPlayerCharacter 0) (Variables|Default|GetTool%20Tip%20Text)))

(event MouseInput|EventActorEndCursorOver
  ;[0.15 0.15 0.15 0.5] Tooltip
  (Class|InteractBPI|SetToolTip(Message) (Game|GetPlayerCharacter 0)))

(fn ConstructionScript)