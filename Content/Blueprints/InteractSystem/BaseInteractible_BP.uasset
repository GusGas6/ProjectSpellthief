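; Base interactible that acts as a switch for the actors in LeverConnectedActors, taking ownership of them on BeginPlay.
; Cursor hover shows a grab cursor, tooltip and looping throb highlight, and spawns cables to each linked actor, expanding TorchMaster_BP into its individual torches.
; Ending hover clears the tooltip and highlight and destroys the cables.
; Interact flip-flops the cube's red/green material and forwards InteractMessage to every valid linked actor.
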(event EventBeginPlay
  (for _array_element (Variables|Default|GetLeverConnectedActors)
    (Actor|SetOwner _array_element self)))

(event MouseInput|EventActorBeginCursorOver
  (Variables|/Script/Engine.PlayerController|SetCurrentMouseCursor (Game|GetPlayerController 0) "GrabHand")
  (Variables|Default|SetMousingOver true)
  (Rendering|SetVisibility (Variables|Default|GetCubeThrob) true false)
  (Utilities|FlowControl|Sequence
    (:then_0
      (bind _newtrack_0 (Timeline|Timeline Play)
        (:Update
          (Transformation|SetWorldScale3D (Variables|Default|GetCubeThrob) (Math|Vector|Lerp(Vector) "1.020000,0.650000,1.020000" "1.200000,0.650000,1.200000" _newtrack_0)))
        (:Finished
          (if (Variables|Default|GetMousingOver)
            (Timeline|Timeline PlayFromStart)))))
    (:then_1
      (for _array_element (Variables|Default|GetLeverConnectedActors)
        (if (== (Utilities|GetClass _array_element) "/Game/Blueprints/Lighting/TorchMaster_BP.TorchMaster_BP_C")
          (bind _astorch_master_bp (Utilities|Casting|CastToTorchMaster_BP _array_element))
          (for _array_element_2 (Variables|/Game/Blueprints/Lighting/TorchMaster_BP.TorchMaster_BP_C|GetTorchLightArray _astorch_master_bp)
            (bind _returnvalue (AddComponent|AddCableComponent true (Math|Transform|MakeTransform (Transformation|GetWorldLocation (Variables|Default|GetCube)) "0, 0, 0" "1.000000,1.000000,1.000000")))
            (Transformation|AttachComponentToComponent _returnvalue (Variables|Default|GetCubeThrob) "None" "SnapToTarget" "KeepWorld" "SnapToTarget" true)
            (Utilities|Array|Add (Variables|Default|GetCableComponents) _returnvalue)
            (Class|CableComponent|SetAttachEndto _returnvalue (Variables|/Script/Engine.ChildActorComponent|GetChildActor _array_element_2) "None" "PushBox"))
          (else
            (bind _returnvalue_2 (AddComponent|AddCableComponent true (Math|Transform|MakeTransform (Transformation|GetWorldLocation (Variables|Default|GetCube)) "0, 0, 0" "1.000000,1.000000,1.000000")))
            (Transformation|AttachComponentToComponent _returnvalue_2 (Variables|Default|GetCubeThrob) "None" "SnapToTarget" "KeepWorld" "SnapToTarget" true)
            (Utilities|Array|Add (Variables|Default|GetCableComponents) _returnvalue_2)
            (Class|CableComponent|SetAttachEndto _returnvalue_2 _array_element "None" "PushBox")))))
    (:then_2
      (Class|InteractBPI|SetToolTip(Message) (Game|GetPlayerCharacter 0) (Variables|Default|GetTool%20Tip%20Text)))))

(event MouseInput|EventActorEndCursorOver
  (bind _cablecomponents (Variables|Default|GetCableComponents))
  (Variables|/Script/Engine.PlayerController|SetCurrentMouseCursor (Game|GetPlayerController 0) "Default")
  (Variables|Default|SetMousingOver false)
  (Rendering|SetVisibility (Variables|Default|GetCubeThrob) false false)
  (Class|InteractBPI|SetToolTip(Message) (Game|GetPlayerCharacter 0))
  (for _array_element _cablecomponents
    (Utilities|IsValid _array_element
      (:Is%20Valid
        (Components|DestroyComponent _array_element))))
  (Utilities|Array|Clear _cablecomponents))

(event EventInteract
  (bind _cube (Variables|Default|GetCube))
  (switch Utilities|FlowControl|Switch|SwitchonInteractibleTypeEnum (Variables|Default|GetInteractibleType)
    (:NewEnumerator0
      (Utilities|FlowControl|FlipFlop
        (:A
          (Rendering|Material|SetMaterial _cube 0 "/AnimationSharing/AnimSharingRed.AnimSharingRed"))
        (:B
          (Rendering|Material|SetMaterial _cube 0 "/AnimationSharing/AnimSharingGreen.AnimSharingGreen")))
      (for _array_element (Variables|Default|GetLeverConnectedActors)
        (Utilities|IsValid _array_element
          (:Is%20Valid
            (Class|InteractBPI|Interact(Message) _array_element)))))))

(fn ConstructionScript)