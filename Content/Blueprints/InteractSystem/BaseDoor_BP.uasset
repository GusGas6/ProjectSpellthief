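; Base interactable door that toggles open or closed on Interact, can start open, and shows a cursor-over tooltip.
; A timeline lerps the mesh rotation, with swing direction set by whether the player character is inside RightBox.
; Collision is disabled on opening and restored once closed, and a random shake plays on bumps and finished swings.
; PushBox sends bump messages to actors hit by the moving door and applies blunt damage to non-players.
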(event OnComponentBeginOverlap(RightBox)
  (params (OverlappedComponent :type Primitive%20Component%20Object%20Reference) (OtherActor :type Actor%20Object%20Reference) (OtherComp :type Primitive%20Component%20Object%20Reference) (OtherBodyIndex :type Integer) (bFromSweep :type Boolean) (SweepResult :type Hit%20Result%20Structure%20%28by%20ref%29))
  (if (== (Utilities|GetClass OtherActor) "/Game/Blueprints/BP_ThirdPersonCharacter.BP_ThirdPersonCharacter_C")
    (Variables|Default|SetRight false)))

(event OnComponentEndOverlap(RightBox)
  (params (OverlappedComponent :type Primitive%20Component%20Object%20Reference) (OtherActor :type Actor%20Object%20Reference) (OtherComp :type Primitive%20Component%20Object%20Reference) (OtherBodyIndex :type Integer))
  (if (== (Utilities|GetClass OtherActor) "/Game/Blueprints/BP_ThirdPersonCharacter.BP_ThirdPersonCharacter_C")
    (Variables|Default|SetRight true)))

(event OnComponentBeginOverlap(PushBox)
  (params (OverlappedComponent :type Primitive%20Component%20Object%20Reference) (OtherActor :type Actor%20Object%20Reference) (OtherComp :type Primitive%20Component%20Object%20Reference) (OtherBodyIndex :type Integer) (bFromSweep :type Boolean) (SweepResult :type Hit%20Result%20Structure%20%28by%20ref%29))
  (if (Variables|Default|GetDoorMoving)
    (Development|PrintString (Utilities|String|Append "DOOR HIT:" (Utilities|GetDisplayName OtherActor)))
    (Class|InteractBPI|Bump(Message) OtherActor false)
    (if (not (== (Game|GetPlayerCharacter 0) OtherActor))
      (Game|Damage|ApplyPointDamage OtherActor 1.0 (Math|Vector|GetUnitDirection(Vector) (Transformation|GetActorLocation) (Transformation|GetActorLocation OtherActor)) SweepResult 0 self "/Game/Blueprints/DamageTypes/Blunt_DamageType.Blunt_DamageType_C"))))

(event Custom|CloseDoor
  (bind _doormesh (Variables|Default|GetDoorMesh))
  (bind _doormesh_2 (Variables|Default|GetDoorMesh))
  (Utilities|Array|RemoveItem (Variables|Actor|GetTags) "open")
  (Variables|Default|SetEndRotation "0, 0, 0")
  (Collision|SetCollisionResponsetoChannel _doormesh "ECC_PhysicsBody" "ECR_Block")
  (Collision|SetCollisionResponsetoChannel _doormesh "ECC_PhysicsBody" "ECR_Overlap")
  (Variables|Default|SetStartRotation (Variables|/Script/Engine.SceneComponent|GetRelativeRotation _doormesh_2))
  (Variables|Default|SetDoorMoving true)
  (bind _newtrack_0 (Timeline|Timeline PlayFromStart)
    (:Update
      (Transformation|SetRelativeRotation _doormesh_2 (Math|Rotator|Lerp(Rotator) (Variables|Default|GetStartRotation) (Variables|Default|GetEndRotation) _newtrack_0 true) false false))
    (:Finished
      (Variables|Default|SetDoorMoving false)
      (CallFunction|DoorShake)
      (if (Utilities|Operators|EqualEqual :A (Variables|Default|GetEndRotation))
        (Collision|SetCollisionEnabled (Variables|Default|GetDoorMesh) "QueryAndPhysics")))))

(event Custom|OpenDoor
  (params (Right :type Boolean))
  (bind _doormesh (Variables|Default|GetDoorMesh))
  (Utilities|Array|Add (Variables|Actor|GetTags) "open")
  (Collision|SetCollisionEnabled (Variables|Default|GetDoorMesh) "NoCollision")
  (if Right
    (Variables|Default|SetEndRotation "0.000000,-90.000000,0.000000")
    (else
      (Variables|Default|SetEndRotation "0.000000,90.000000,0.000000")))
  (Collision|SetCollisionResponsetoChannel (Variables|Default|GetDoorMesh) "ECC_PhysicsBody" "ECR_Overlap")
  (Variables|Default|SetStartRotation (Variables|/Script/Engine.SceneComponent|GetRelativeRotation _doormesh))
  (Variables|Default|SetDoorMoving true)
  (bind _newtrack_0 (Timeline|Timeline PlayFromStart)
    (:Update
      (Transformation|SetRelativeRotation _doormesh (Math|Rotator|Lerp(Rotator) (Variables|Default|GetStartRotation) (Variables|Default|GetEndRotation) _newtrack_0 true) false false))
    (:Finished
      (Variables|Default|SetDoorMoving false)
      (CallFunction|DoorShake)
      (if (Utilities|Operators|EqualEqual :A (Variables|Default|GetEndRotation))
        (Collision|SetCollisionEnabled (Variables|Default|GetDoorMesh) "QueryAndPhysics")))))

(event Custom|DoorShake
  (Variables|Default|SetRandomShakeVector (Math|Vector|MakeVector (Math|Random|RandomFloatinRange -25.0 25.0) (Math|Random|RandomFloatinRange -25.0 25.0) (Math|Random|RandomFloatinRange -25.0 25.0)))
  (bind _newtrack_0 (Timeline|Timeline_0 PlayFromStart)
    (:Update
      (Transformation|SetRelativeLocation (Variables|Default|GetDoorShaker) (Math|Vector|Lerp(Vector) "0, 0, 0" (Math|Vector|MakeVector (.x (Variables|Default|GetRandomShakeVector)) 0.0 (.z (Variables|Default|GetRandomShakeVector))) _newtrack_0) false false))))

(event EventBump
  (params (ON :type Boolean))
  (CallFunction|DoorShake))

(event EventBeginPlay)

(event EventInteract
  (Utilities|FlowControl|FlipFlop
    (:A
      (if (Variables|Default|GetStartOpen)
        (CallFunction|CloseDoor :!label _label)
        (else
          (CallFunction|OpenDoor (Variables|Default|GetRight) :!label _label_2))))
    (:B
      (if (Variables|Default|GetStartOpen)
        (goto _label_2)
        (else
          (goto _label))))))

(event MouseInput|EventActorBeginCursorOver
  ;[0.15 0.15 0.15 0.5] Tooltip
  (Class|InteractBPI|SetToolTip(Message) (Game|GetPlayerCharacter 0) (Variables|Default|GetTool%20Tip%20Text)))

(event MouseInput|EventActorEndCursorOver
  ;[0.15 0.15 0.15 0.5] Tooltip
  (Class|InteractBPI|SetToolTip(Message) (Game|GetPlayerCharacter 0)))

(event EventRequestInfo
  (params (RequestOrigin :type Actor%20Object%20Reference) (ConnectedLever :type Actor%20Object%20Reference))
  (Class|InteractBPI|RequestInfo(Message) RequestOrigin 0 (Components|GetOwner)))

(fn ConstructionScript
  (if (Variables|Default|GetStartOpen)
    (if (Variables|Default|GetRight)
      (Variables|Default|SetEndRotation "0.000000,-90.000000,0.000000")
      (else
        (Variables|Default|SetEndRotation "0.000000,90.000000,0.000000")))
    (Transformation|SetRelativeRotation (Variables|Default|GetDoorMesh) (Variables|Default|GetEndRotation) false false)))