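; Base Blueprint for gib debris actors that clean themselves up after spawning.
; After a custom lifetime, a timeline shrinks the actor to zero scale and then destroys it.
; In parallel, a looping delay polls mesh velocity and switches off physics simulation once the gib is nearly at rest.
; BeginPlay also sets the first player character as the gib's owner.
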(event EventBeginPlay
  (Utilities|FlowControl|Sequence
    (:then_0
      (Utilities|FlowControl|Delay (Variables|Default|GetCustomGibLifetime))
      (Variables|Default|SetActorScale (Transformation|GetActorScale3D))
      (bind _newtrack_0 (Timeline|Timeline PlayFromStart)
        (:Update
          (Transformation|SetActorScale3D (Math|Vector|Lerp(Vector) (Variables|Default|GetActorScale) "0, 0, 0" _newtrack_0)))
        (:Finished
          (Actor|DestroyActor))))
    (:then_1
      (Utilities|FlowControl|Delay 2.0 :!label _label)
      (if (Utilities|Operators|EqualEqual :A (Transformation|GetComponentVelocity (Variables|Default|GetBaseGibMesh)) :ErrorTolerance 5.0)
        (Physics|SetSimulatePhysics (Variables|Default|GetBaseGibMesh) false)
        (else
          (goto _label))))
    (:then_2
      (Actor|SetOwner (Game|GetPlayerCharacter 0)))))

(fn ConstructionScript)