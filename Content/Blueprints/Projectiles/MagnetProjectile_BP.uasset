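; Magnet projectile that homes back to the player with timeline-ramped acceleration and destroys itself on contact with them.
; On overlapping a BaseAI_BP with pickpocket data, it hooks once onto the AI's MagnetHookLocation and sends the player a clamped tether distance.
; A per-tick loop pins it to the hook until the player exceeds that distance plus some slack, then reattaches the mesh to the sphere, freeing it to return.
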(event OnComponentBeginOverlap(Sphere)
  (params (OverlappedComponent :type Primitive%20Component%20Object%20Reference) (OtherActor :type Actor%20Object%20Reference) (OtherComp :type Primitive%20Component%20Object%20Reference) (OtherBodyIndex :type Integer) (bFromSweep :type Boolean) (SweepResult :type Hit%20Result%20Structure%20%28by%20ref%29))
  (bind _returnvalue (Game|GetPlayerCharacter 0))
  (bind _magnetmesh (Variables|Default|GetMagnetMesh))
  (bind _returnvalue_2 (Transformation|GetWorldLocation _magnetmesh))
  (bind _returnvalue_3 (Transformation|GetActorLocation _returnvalue))
  (bind _returnvalue_4 (Math|Vector|Distance(Vector) _returnvalue_2 _returnvalue_3))
  (if (== OtherActor (Game|GetPlayerCharacter 0))
    (Actor|DestroyActor)
    (elif (== (Utilities|GetClass OtherActor) "/Game/Blueprints/AI/BaseAI_BP.BaseAI_BP_C")
      (bind _asbase_ai_bp (Utilities|Casting|CastToBaseAI_BP OtherActor))
      (if (not (== (Variables|/Game/Blueprints/AI/BaseAI_BP.BaseAI_BP_C|GetPickPocket_DA _asbase_ai_bp) 0))
        (Utilities|FlowControl|DoOnce false
          (:Completed
            (Transformation|AttachComponentToComponent _magnetmesh (Variables|/Game/Blueprints/AI/BaseAI_BP.BaseAI_BP_C|GetMagnetHookLocation _asbase_ai_bp) "None" "SnapToTarget" "SnapToTarget" "KeepWorld" true)
            (Variables|Default|SetStoredDistance (Math|Float|Clamp(Float) _returnvalue_4 2e+02 5.5e+02))
            (Variables|Default|SetHooked true)
            (Utilities|FlowControl|Sequence
              (:then_0
                (Class|PickpocketingBPI|StoredDistanceBump(Message) _returnvalue (* (Variables|Default|GetStoredDistance) 1.15) (Variables|Default|GetStoredDistance) self _magnetmesh))
              (:then_1
                (Transformation|SetActorLocation (Transformation|GetWorldLocation (Variables|/Game/Blueprints/AI/BaseAI_BP.BaseAI_BP_C|GetMagnetHookLocation _asbase_ai_bp)) false true :!label _label)
                (Variables|/Script/Engine.MovementComponent|SetVelocity (Variables|Default|GetProjectileMovement) "0, 0, 0")
                (if (< _returnvalue_4 (* (Variables|Default|GetStoredDistance) 1.15))
                  (if (Variables|Default|GetHooked)
                    (Utilities|FlowControl|DelayUntilNextTick)
                    (goto _label))
                  (else
                    (Variables|Default|SetHooked false)
                    (Utilities|IsValid (Variables|/Game/Blueprints/AI/BaseAI_BP.BaseAI_BP_C|GetMagnetHookLocation _asbase_ai_bp)
                      (:Is%20Valid
                        (Transformation|AttachComponentToComponent (Variables|Default|GetMagnetMesh) (Variables|Default|GetSphere) "None" "SnapToTarget" "KeepWorld" "KeepWorld" true)
                        (Variables|/Script/Engine.ProjectileMovementComponent|SetbRotationFollowsVelocity (Variables|Default|GetProjectileMovement) false)))))))))))))

(event EventBeginPlay
  (bind _projectilemovement (Variables|Default|GetProjectileMovement))
  (Utilities|FlowControl|Sequence
    (:then_0
      (Utilities|FlowControl|Delay 0.1)
      (Collision|SetCollisionResponsetoChannel (Variables|Default|GetSphere) "ECC_GameTraceChannel3" "ECR_Overlap"))
    (:then_1
      (Variables|/Script/Engine.ProjectileMovementComponent|SetHomingTargetComponent _projectilemovement (Variables|/Script/Engine.Actor|GetRootComponent (Game|GetPlayerCharacter 0)))
      (Variables|/Script/Engine.ProjectileMovementComponent|SetbIsHomingProjectile _projectilemovement true)
      (bind _newtrack_0 (Timeline|Timeline PlayFromStart)
        (:Update
          (Variables|/Script/Engine.ProjectileMovementComponent|SetHomingAccelerationMagnitude (Variables|Default|GetProjectileMovement) (Math|Float|Lerp 0.0 99999.0 _newtrack_0)))))
    (:then_2
      (Variables|Default|SetCustomTimeDilation 0.75)
      (Actor|SetOwner (Game|GetPlayerCharacter 0)))))

(fn ConstructionScript)