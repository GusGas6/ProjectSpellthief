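; Base projectile actor that takes its speed, damage type, collision radius, trail and impact effect from a ProjectileTypeDA data asset.
; BeginPlay launches it along its forward vector, then waits a tick before making collision block Pawns and zeroing the trail's relative location.
; On hit it prints the struck component, applies fixed point damage, spawns the impact emitter, disables collision and destroys itself after a short delay.
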(event EventBeginPlay
  (bind _projectilemovement (Variables|Default|GetProjectileMovement))
  (bind _projectiletype_da (Variables|Default|GetProjectileType_DA))
  (Utilities|FlowControl|Sequence
    (:then_0
      (Variables|/Script/Engine.ProjectileMovementComponent|SetMaxSpeed _projectilemovement (Variables|/Game/Blueprints/DataAssets/Enemies/ProjectileType_DA.ProjectileType_DA_C|GetMax%20Speed _projectiletype_da))
      (Variables|/Script/Engine.MovementComponent|SetVelocity _projectilemovement (* (Transformation|GetActorForwardVector) (Variables|/Game/Blueprints/DataAssets/Enemies/ProjectileType_DA.ProjectileType_DA_C|GetVelocityMultiplier _projectiletype_da)))
      (Variables|Default|SetDamage%20Type%20Class (Variables|/Game/Blueprints/DataAssets/Enemies/ProjectileType_DA.ProjectileType_DA_C|GetDamage%20Type%20Class _projectiletype_da))
      (Class|NiagaraComponent|SetAsset (Variables|Default|GetTrail) (Variables|/Game/Blueprints/DataAssets/Enemies/ProjectileType_DA.ProjectileType_DA_C|GetTrail _projectiletype_da) true)
      (Components|Sphere|SetSphereRadius (Variables|Default|GetCollision) (Variables|/Game/Blueprints/DataAssets/Enemies/ProjectileType_DA.ProjectileType_DA_C|GetCollisionRadius _projectiletype_da) true))
    (:then_1
      (Utilities|FlowControl|DelayUntilNextTick)
      (Collision|SetCollisionResponsetoChannel (Variables|Default|GetCollision) "ECC_Pawn" "ECR_Block")
      (Transformation|SetRelativeLocation (Variables|Default|GetTrail) "0, 0, 0" false false))))

(event Collision|EventHit
  (params (MyComp :type Primitive%20Component%20Object%20Reference) (Other :type Actor%20Object%20Reference) (OtherComp :type Primitive%20Component%20Object%20Reference) (bSelfMoved :type Boolean) (HitLocation :type Vector :default "0, 0, 0") (HitNormal :type Vector :default "0, 0, 0") (NormalImpulse :type Vector :default "0, 0, 0") (Hit :type Hit%20Result%20Structure%20%28by%20ref%29))
  (Development|PrintString (Utilities|GetDisplayName OtherComp))
  (Game|Damage|ApplyPointDamage Other 1.0 (Math|Vector|GetUnitDirection(Vector) (Transformation|GetActorLocation) HitLocation) Hit 0 self (Variables|Default|GetDamage%20Type%20Class))
  (Effects|SpawnEmitteratLocation (Variables|/Game/Blueprints/DataAssets/Enemies/ProjectileType_DA.ProjectileType_DA_C|GetImpactVFX (Variables|Default|GetProjectileType_DA)) HitLocation (Math|Conversions|RotationFromXVector HitNormal) "0.400000,0.400000,0.400000")
  (Collision|SetCollisionEnabled (Variables|Default|GetCollision) "NoCollision")
  (Utilities|FlowControl|Delay 0.4)
  (Actor|DestroyActor))

(fn ConstructionScript)